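; Base enemy character Blueprint that links an AI controller, a damage system component and a health bar widget.
; Health, healing and damage calls pass through to the component, whose death and damage-response delegates drive destruction and hit reactions.
; A hit freezes the AI during a montage, then resumes attacking the last known target.
; It exposes patrol route, combat ranges and movement speed to callers, with Attack and IsDead left as stubs.
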(event Custom|Die
  (AI|Logic|StopLogic (Variables|/Script/AIModule.AIController|GetBrainComponent (Variables|Default|GetAIC%20Enemy%20Base)) "")
  (Default|SetStateasDead (Variables|Default|GetAIC%20Enemy%20Base))
  (Actor|DestroyActor))

(event Custom|HitResponse
  (params (DamageResponse :type E_DamageResponse%20Enum :default "NewEnumerator0"))
  (Components|Movement|StopMovementImmediately (Variables|Character|GetCharacterMovement))
  (Default|SetStateasFrozen (Variables|Default|GetAIC%20Enemy%20Base))
  (Animation|Montage|PlayMontage (Variables|Character|GetMesh) (Variables|Default|GetHitReactionMontage)
    (:OnCompleted
      (Default|SetStateasAttacking (Variables|Default|GetAIC%20Enemy%20Base) 0 true))))

(event EventBeginPlay
  (bind _bpc_damagesystem (Variables|Default|GetBPC_DamageSystem))
  (bind _asaic_enemy_base (Utilities|Casting|CastToAIC_Enemy_Base (AI|GetAIController self)))
  (Variables|Default|SetAIC%20Enemy%20Base _asaic_enemy_base)
  (bind _returnvalue (UserInterface|CreateWidget "/Game/DamageSystem/W_HealthBar.W_HealthBar_C" 0 self))
  (UserInterface|SetWidget (Variables|Default|GetHealthBar) _returnvalue)
  (EventDispatchers|AssignOnDeath _bpc_damagesystem (EventDispatchers|CreateEvent :!event Custom|Die))
  (EventDispatchers|AssignOnDamageResponse _bpc_damagesystem (EventDispatchers|CreateEvent :!event Custom|HitResponse)))

(fn ConstructionScript)

(fn Attack
  (return))

(fn GetCurrentHealth
  (return (Variables|/Game/DamageSystem/BPC_DamageSystem.BPC_DamageSystem_C|GetHealth (Variables|Default|GetBPC_DamageSystem))))

(fn GetIdealRange
  (return 2e+02 3.5e+02))

(fn GetMaxHealth
  (return (Variables|/Game/DamageSystem/BPC_DamageSystem.BPC_DamageSystem_C|GetMaxHealth (Variables|Default|GetBPC_DamageSystem))))

(fn GetPatrolRoute
  (return (Variables|AI|GetPatrolRoute)))

(fn Heal
  (params (Amount :type Float%20%28double-precision%29))
  (bind _newhealth (Default|Heal (Variables|Default|GetBPC_DamageSystem) Amount))
  (return _newhealth))

(fn IsAttack
  (return (Variables|Default|GetAttacking)))

(fn IsDead
  (return false))

(fn SetMovementSpeed
  (params (Speed :type E_MovementSpeed%20Enum :default "NewEnumerator0"))
  (bind _output_get (Variables|/Script/Engine.CharacterMovementComponent|SetMaxWalkSpeed (Variables|Character|GetCharacterMovement) (Utilities|Select :Index Speed :NewEnumerator0 0.0 :NewEnumerator1 3e+02 :NewEnumerator2 6e+02)))
  (return _output_get))

(fn TakeDamage
  (params (DamageInfo :type S%20Damage%20Info%20Structure))
  (bind _wasdamaged (Default|TakeDamage (Variables|Default|GetBPC_DamageSystem) DamageInfo))
  (return _wasdamaged))