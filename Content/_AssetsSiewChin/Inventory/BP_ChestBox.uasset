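; BP_ChestBox is an interactable chest that opens its lid when a valid player interacts with it.
; OnInteracted calls OpenChest, which plays a timeline that lerps the roll of the ChestTop mesh to swing it open.
; OnHovered sets custom depth and stencil on both chest parts, but its hardcoded false inputs turn custom depth off and select a zero stencil.
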(event Custom|OpenChest
  (bind _chesttop (Variables|Default|GetChestTop))
  (bind _relativerotation (Variables|/Script/Engine.SceneComponent|GetRelativeRotation _chesttop))
  (bind _lerpvalue (Timeline|Timeline_OpenChest Play)
    (:Update
      (Transformation|SetRelativeRotation _chesttop (Math|Rotator|MakeRotator (Math|Float|Lerp 0.0 1.1e+02 _lerpvalue) (.pitch _relativerotation) (.yaw _relativerotation)) false false))))

(event EventOnInteracted
  (params (PlayerRef :type Main%20Player%201%20Object%20Reference))
  (Utilities|IsValid PlayerRef
    (:Is%20Valid
      (CallFunction|OpenChest))))

(event EventOnHovered
  (params (bisHovered? :type Boolean) (Player%20Ref :type Main%20Player%201%20Object%20Reference))
  (Rendering|SetRenderCustomDepth (Variables|Default|GetChestTop) false)
  (Rendering|SetCustomDepthStencilValue (Variables|Default|GetChestTop) (Math|Integer|SelectInt 1 0 false)))

(fn ConstructionScript)