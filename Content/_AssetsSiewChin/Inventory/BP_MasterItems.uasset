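; BP_MasterItems is an interactable pickup item, apparently a base for inventory items.
; On hover it toggles an outline on its static mesh through custom depth rendering and a stencil value.
; On interaction it passes the player to the chest HUD's UpdateItemsCounts, then destroys itself.
; Both events act only when the player reference is valid.
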(event EventOnInteracted
  (params (PlayerRef :type Tan%20Hao%20Main%20Player%20Object%20Reference))
  ;[0.15 0.15 0.15 0.5] Interaction Event
  (Utilities|IsValid PlayerRef
    (:Is%20Valid
      (Default|UpdateItemsCounts (Variables|/Game/_AssetsTanHao/Player_TanHao/TanHaoMainPlayer.TanHaoMainPlayer_C|GetPlayerHudChest PlayerRef) PlayerRef)
      (Actor|DestroyActor))))

(event EventOnHovered
  (params (bisHovered? :type Boolean) (Player%20Ref :type Tan%20Hao%20Main%20Player%20Object%20Reference))
  ;[0.15 0.15 0.15 0.5] Interaction Event
  (Utilities|IsValid Player%20Ref
    (:Is%20Valid
      (CallFunction|ToggleOutline bisHovered?))))

(fn ConstructionScript)

(fn ToggleOutline
  (params (Isvisible?%20 :type Boolean))
  (bind _staticmesh (Variables|Default|GetStaticMesh))
  (Rendering|SetRenderCustomDepth _staticmesh Isvisible?%20)
  (Rendering|SetCustomDepthStencilValue _staticmesh (Math|Integer|SelectInt 1 0 Isvisible?%20)))