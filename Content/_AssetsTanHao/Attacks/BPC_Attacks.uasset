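; Attack component that gives its owning actor a hitscan bullet and a dark-energy magic projectile.
; FireBullet line-traces for Pawns, while MagicSpell spawns a targeted projectile, binds its impact event and has the owner's capsule ignore it.
; Both deliver damage through the TakeDamage message and report a damage event crediting the owner as instigator.
; Only the projectile impact calls OnAttackEnded.
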(event Custom|MagicSpell
  (params (SpawnTransform :type Transform) (Target :type Actor%20Object%20Reference) (DamageInfo :type S%20Damage%20Info%20Structure))
  (bind _returnvalue (Game|SpawnActorfromClass "/Game/_AssetsTanHao/Projectiles/BP_Projectile_DarkEnergy.BP_Projectile_DarkEnergy_C" SpawnTransform "Undefined" "MultiplyWithRoot" (Components|GetOwner) 2e+03 0.0 Target false 0))
  (EventDispatchers|BindEventtoOnProjectileImpact _returnvalue (delegate Custom|OnProjectHit))
  (Collision|IgnoreActorwhenMoving (Actor|GetComponentbyClass (Components|GetOwner) "/Script/Engine.CapsuleComponent") _returnvalue true))

(event Custom|OnProjectHit
  (params (Other%20Actor :type Actor%20Object%20Reference) (Hit :type Hit%20Result%20Structure))
  (Class|BPIDamagable|TakeDamage(Message) Other%20Actor (stale Custom|MagicSpell DamageInfo))
  (Class|AISenseDamage|ReportDamageEvent Other%20Actor (Components|GetOwner) (Utilities|Struct|BreakS_DamageInfo (stale Custom|MagicSpell DamageInfo)) (Transformation|GetActorLocation (Components|GetOwner)) "0, 0, 0" "None")
  (Default|CallOnAttackEnded))

(event Custom|FireBullet
  (params (TraceStart :type Vector) (TraceEnd :type Vector) (DamageInfo :type S%20Damage%20Info%20Structure))
  (bind (_outhit _returnvalue) (Collision|LineTraceForObjects TraceStart TraceEnd (Utilities|Array|MakeArray "ObjectTypeQuery3") false 0 "None"))
  (if _returnvalue
    (Class|BPIDamagable|TakeDamage(Message) (.HitActor (Collision|BreakHitResult _outhit)) DamageInfo)
    (Class|AISenseDamage|ReportDamageEvent (.HitActor (Collision|BreakHitResult _outhit)) (Components|GetOwner) (Utilities|Struct|BreakS_DamageInfo DamageInfo) (Transformation|GetActorLocation (Components|GetOwner)) "0, 0, 0" "None")))